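; Game instance for the Island game that holds the turn counter and the list of people.
; CreatePerson spawns a Hairdresser or Mime actor by ID at the world origin, adds it to People and returns it.
; EndTurn increments Turn and broadcasts it through OnEndTurn.
; SwitchScene is a stub with an empty switch on Scene, alongside unconnected level-opening and streaming-instance nodes.
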(fn CreatePerson
  (params (Id :type String))
  (switch string Id
    (:Default
      _)
    (:Hairdresser
      (bind _returnvalue (Game|SpawnActorfromClass "/Game/Island/Blueprints/Actor/People/BP_Person_Hairdresser.BP_Person_Hairdresser_C" (Math|Transform|MakeTransform "0, 0, 0") "Undefined" 0 0))
      (LocalVariables|SetCreatePerson_CreatedPerson _returnvalue)
      (Utilities|Array|Add (LocalVariables|GetPeople) (LocalVariables|GetCreatePerson_CreatedPerson) :!label _label))
    (:Mime
      (bind _returnvalue_2 (Game|SpawnActorfromClass "/Game/Island/Blueprints/Actor/People/BP_Person_Mime.BP_Person_Mime_C" (Math|Transform|MakeTransform "0, 0, 0") "Undefined" 0 0))
      (LocalVariables|SetCreatePerson_CreatedPerson _returnvalue_2)
      (goto _label)))
  (return (LocalVariables|GetCreatePerson_CreatedPerson)))

(fn SwitchScene
  (params (Scene :type Enum_Scene%20Enum))
  (switch Utilities|FlowControl|Switch|SwitchonEnum_Scene Scene))

(fn EndTurn
  (bind _turn (Variables|Default|GetTurn))
  (Math|Integer|IncrementInt _turn
    (:%20%20
      (Default|CallOnEndTurn _turn))))