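; Camp HUD that builds the island camp screen: layout, placeables panel and an End turn button that currently only prints.
; On BeginPlay it creates a person through GI_Island, adds their token widget and opens their exploration window.
; Tick projects each token's assigned actor location to screen to position the token.
; Helpers size overlay widgets to placeables' screen bounds, but their update call and the debug bounds drawing are disconnected.
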(event Custom|_ButtonOnClicked
  (params (NewParam :type String))
  (Utilities|Casting|CastToGI_Island (Game|GetGameInstance))
  (Development|PrintString "End turn"))

(event EventBeginPlay
  (bind _returnvalue (Game|GetPlayerController 0))
  (Utilities|FlowControl|Sequence
    (:then_0
      (bind _returnvalue_2 (UserInterface|CreateWidget "/Game/Island/Blueprints/Widgets/Layout/Widget_CampLayout.Widget_CampLayout_C" (Game|GetPlayerController 0)))
      (UserInterface|Viewport|AddtoViewport _returnvalue_2 0)
      (Utilities|FlowControl|Sequence
        (:then_0
          (bind _returnvalue_3 (UserInterface|CreateWidget "/Game/Island/Blueprints/Widgets/Widget_Placeables.Widget_Placeables_C" _returnvalue))
          (Widget|Panel|AddChild (Variables|/Game/Island/Blueprints/Widgets/Layout/Widget_CampLayout.Widget_CampLayout_C|GetBottomLeftSlot _returnvalue_2) _returnvalue_3))
        (:then_1
          (bind _returnvalue_4 (UserInterface|CreateWidget "/Game/Island/Blueprints/Widgets/Blocks/WB_Button.WB_Button_C" _returnvalue "End turn"))
          (Widget|Panel|AddChild (Variables|/Game/Island/Blueprints/Widgets/Layout/Widget_CampLayout.Widget_CampLayout_C|GetBottomRightSlot _returnvalue_2) _returnvalue_4)
          (EventDispatchers|BindEventtoButtononClicked _returnvalue_4 (delegate Custom|_ButtonOnClicked)))))
    (:then_2
      ;[1 1 1] Create person and their token widget
      (bind _asgi_island (Utilities|Casting|CastToGI_Island (Game|GetGameInstance)))
      (bind _person (Default|CreatePerson _asgi_island "None"))
      (bind _returnvalue_5 (UserInterface|CreateWidget "/Game/Island/Blueprints/Widgets/Widget_Token.Widget_Token_C" (Game|GetPlayerController 0) "1" 0 _person))
      (UserInterface|Viewport|AddtoViewport _returnvalue_5 0)
      (Utilities|Array|Add (Variables|Default|GetTokens) _returnvalue_5)
      (CallFunction|OpenExploration _person))))

(event EventTick
  (params (DeltaSeconds :type Float%20%28single-precision%29))
  (CallFunction|UpdateTokenPlacements))

(event EventDrawHUD
  (params (SizeX :type Integer) (SizeY :type Integer)))

(fn ConstructionScript)

(fn UpdateTokenPlacements
  (for _array_element (Variables|Default|GetTokens)
    (if (!= (Variables|/Game/Island/Blueprints/Widgets/Widget_Token.Widget_Token_C|GetAsignedTo _array_element) 0)
      (Class|UserWidget|SetPositioninViewport _array_element (.ScreenPosition (Class|GameplayStatics|ProjectWorldtoScreen (Game|GetPlayerController 0) (Transformation|GetActorLocation (Variables|/Game/Island/Blueprints/Widgets/Widget_Token.Widget_Token_C|GetAsignedTo _array_element)))) true)
      (else
        (Class|UserWidget|SetPositioninViewport _array_element "(X=0.000000,Y=0.000000)" true)))))

(fn CreatePlaceableSpace
  (params (Placeable :type BP%20Placeable%20Object%20Reference))
  (bind _aspc_camp_controller (Utilities|Casting|CastToPC_CampController (Game|GetPlayerController 0)))
  (bind _returnvalue (UserInterface|CreateWidget "/Game/Island/Blueprints/Widgets/Widget_PlaceableSpace.Widget_PlaceableSpace_C" _aspc_camp_controller Placeable))
  (UserInterface|Viewport|AddtoViewport _returnvalue 0)
  (Class|UserWidget|SetPositioninViewport _returnvalue (.Min (Utilities|Struct|BreakBox2D (Class|IslandPlayerControllerBase|GetObjectScreenBounds _aspc_camp_controller Placeable))) true)
  (Class|UserWidget|SetDesiredSizeinViewport _returnvalue (- (.Max (Utilities|Struct|BreakBox2D (Class|IslandPlayerControllerBase|GetObjectScreenBounds _aspc_camp_controller Placeable))) (.Min (Utilities|Struct|BreakBox2D (Class|IslandPlayerControllerBase|GetObjectScreenBounds _aspc_camp_controller Placeable)))))
  (Utilities|Array|Add (Variables|Default|GetPlaceableSpaces) _returnvalue))

(fn UpdatePlaceableSpaces
  (bind _aspc_camp_controller (Utilities|Casting|CastToPC_CampController (Game|GetPlayerController 0)))
  (for _array_element (Variables|Default|GetPlaceableSpaces)
    (Class|UserWidget|SetPositioninViewport _array_element (.Min (Utilities|Struct|BreakBox2D (Class|IslandPlayerControllerBase|GetObjectScreenBounds _aspc_camp_controller (Variables|/Game/Island/Blueprints/Widgets/Widget_PlaceableSpace.Widget_PlaceableSpace_C|GetPlaceable _array_element)))) true)
    (Class|UserWidget|SetDesiredSizeinViewport _array_element (- (.Max (Utilities|Struct|BreakBox2D (Class|IslandPlayerControllerBase|GetObjectScreenBounds _aspc_camp_controller (Variables|/Game/Island/Blueprints/Widgets/Widget_PlaceableSpace.Widget_PlaceableSpace_C|GetPlaceable _array_element)))) (.Min (Utilities|Struct|BreakBox2D (Class|IslandPlayerControllerBase|GetObjectScreenBounds _aspc_camp_controller (Variables|/Game/Island/Blueprints/Widgets/Widget_PlaceableSpace.Widget_PlaceableSpace_C|GetPlaceable _array_element))))))))

(fn OpenExploration
  (params (Person :type BP%20Person%20Object%20Reference))
  (if (!= Person 0)
    (bind _returnvalue (UserInterface|CreateWidget "/Game/Island/Blueprints/Widgets/Widget_ExplorationWindow.Widget_ExplorationWindow_C" (Game|GetPlayerController 0) Person))
    (UserInterface|Viewport|AddtoViewport _returnvalue 0)))