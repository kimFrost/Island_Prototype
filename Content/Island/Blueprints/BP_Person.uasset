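; Island villager character that gets a random profession and two distinct random traits in its construction script.
; Game Instance events make it process its states and reset per-turn data on each new turn.
; GoToNewSlot swaps its two-way slot link and flags Tick to AI-move there; Tick also draws states and name as debug text.
; Select tints the dynamic body material and deselects all other people, but click events don't call it.
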(event OnClicked(Mesh)
  (params (TouchedComponent :type Primitive%20Component%20Object%20Reference) (ButtonPressed :type Key%20Structure :default "AnyKey")))

(event OnClicked(CapsuleComponent)
  (params (TouchedComponent :type Primitive%20Component%20Object%20Reference) (ButtonPressed :type Key%20Structure :default "AnyKey")))

(event Custom|_OnProcessPeople
  (Class|IslandPerson|ProcessStates))

(event Custom|_OnNewTurn
  (params (Turn :type Integer))
  (Variables|Default|SetbEatenThisTurn false)
  (Utilities|Array|Clear (Variables|Default|GetTasksDoneThisTurn)))

(event EventDestroyed
  ;[1 1 1] Remove self from asigned
  (Variables|/Game/Island/Blueprints/Actor/Components/C_StationSlot.C_StationSlot_C|SetAsignedPerson (Variables|Default|GetAsignedSlot) 0))

(event EventBeginPlay
  (|CallParentFunction)
  (bind _asgi_island (Utilities|Casting|CastToGI_Island (Game|GetGameInstance)))
  (EventDispatchers|BindEventtoOnProcessPeople _asgi_island (delegate Custom|_OnProcessPeople))
  (EventDispatchers|BindEventtoOnNewTurn _asgi_island (delegate Custom|_OnNewTurn)))

(event EventActorBeginOverlap
  (params (OtherActor :type Actor%20Object%20Reference)))

(event EventTick
  (params (DeltaSeconds :type Float%20%28single-precision%29))
  (Utilities|FlowControl|Sequence
    (:then_0
      ;[1 1 1] Simple move between stations
      (if (Variables|Default|GetIsAsignedSlotChanged)
        (Variables|Default|SetIsAsignedSlotChanged false)
        (bind _movementresult (AI|AIMoveTo self (Transformation|GetWorldLocation (Variables|Default|GetAsignedSlot)) 0 5.0 false)
          (:then
            (Variables|Default|SetIsMoving true))
          (:OnSuccess
            (Variables|Default|SetIsMoving false))
          (:OnFail
            (Variables|Default|SetIsMoving false)))))
    (:then_1
      (for (_array_element _array_index) (Variables|Default|GetStates)
        (Rendering|Debug|DrawDebugString (+ (* "0, 0,50.000000" _array_index) (Transformation|GetActorLocation)) (Utilities|String|EnumtoString _array_element) 0 "(R=0.564425,G=0.000000,B=1.000000,A=1.000000)")))
    (:then_2
      (Rendering|Debug|DrawDebugString (+ (Transformation|GetActorLocation) "0, 0,-50.000000") (Variables|Default|GetFirstName) 0 "(R=0.564425,G=0.000000,B=1.000000,A=1.000000)"))))

(fn ConstructionScript
  (|CallParentFunction)
  (CallFunction|CreateRandom)
  (bind _returnvalue (Rendering|Material|CreateDynamicMaterialInstance (Variables|Character|GetMesh) 0 (Rendering|Material|GetMaterial (Variables|Character|GetMesh) 0) :!class /Script/Engine.PrimitiveComponent))
  (bind _output_get (Variables|Default|SetDynamicMaterialBody _returnvalue))
  (Rendering|Material|SetVectorParameterValue _output_get "BodyColor" "(R=0.865000,G=0.865000,B=0.865000,A=1.000000)" :!class /Script/Engine.MaterialInstanceDynamic))

(fn CreateRandom
  (Utilities|FlowControl|Sequence
    (:then_0
      (bind _outrownames (DataTable|GetDataTableRowNames "/Game/Island/Util/Structs/DATA_Professions.DATA_Professions"))
      (bind _returnvalue (Utilities|GetDataTableRow "/Game/Island/Util/Structs/DATA_Professions.DATA_Professions" (Utilities|Array|Get(acopy) _outrownames (Math|Random|RandomIntegerinRange 0 (- (Utilities|Array|Length _outrownames) 1))))
        (:then
          (Variables|Default|SetProfession _returnvalue))))
    (:then_1
      (Utilities|Array|Clear (Variables|Default|GetTraits))
      (for _index (range 0 1)
        (bind _trait (CallFunction|GetNewRandomTrait))
        (Utilities|Array|Add (Variables|Default|GetTraits) _trait)))))

(fn GetNewRandomTrait
  (bind _outrownames (DataTable|GetDataTableRowNames "/Game/Island/Util/Structs/DATA_Traits_DEPRECATED.DATA_Traits_DEPRECATED"))
  (bind _returnvalue (Utilities|GetDataTableRow "/Game/Island/Util/Structs/DATA_Traits_DEPRECATED.DATA_Traits_DEPRECATED" (Utilities|Array|Get(acopy) _outrownames (Math|Random|RandomIntegerinRange 0 (- (Utilities|Array|Length _outrownames) 1))))
    (:then
      (if (Utilities|Array|ContainsItem (Variables|Default|GetTraits) _returnvalue)
        (bind _trait (CallFunction|GetNewRandomTrait))
        (return _trait)
        (else
          (return _returnvalue))))
    (:RowNotFound
      (return ""))))

(fn Select
  (bind _outactors (Actor|GetAllActorsOfClass "BP_Person_C"))
  (for _array_element _outactors
    (if (== _array_element self)
      (Rendering|Material|SetVectorParameterValue (Variables|Default|GetDynamicMaterialBody) "BodyColor" "(R=0.414740,G=0.865000,B=0.376275,A=1.000000)" :!class /Script/Engine.MaterialInstanceDynamic)
      (Variables|Default|SetIsSelected true)
      (else
        (CallFunction|Deselect _array_element)))))

(fn Deselect
  (Rendering|Material|SetVectorParameterValue (Variables|Default|GetDynamicMaterialBody) "BodyColor" "(R=0.865000,G=0.865000,B=0.865000,A=1.000000)" :!class /Script/Engine.MaterialInstanceDynamic)
  (Variables|Default|SetIsSelected false))

(fn GotoNewSlot
  (params (Slot :type C%20Station%20Slot%20Object%20Reference))
  (Class|IslandBlueprintFunctionLibrary|NotNull Slot
    (:Exits
      (Class|IslandBlueprintFunctionLibrary|NotNull (Variables|Default|GetAsignedSlot)
        (:Exits
          (Variables|/Game/Island/Blueprints/Actor/Components/C_StationSlot.C_StationSlot_C|SetAsignedPerson (Variables|Default|GetAsignedSlot) 0))
        (:Null
          _))
      (bind _output_get (Variables|Default|SetAsignedSlot Slot))
      (Variables|/Game/Island/Blueprints/Actor/Components/C_StationSlot.C_StationSlot_C|SetAsignedPerson _output_get self)
      (Variables|Default|SetIsAsignedSlotChanged true))))