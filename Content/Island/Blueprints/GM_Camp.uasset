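; GM_Camp is the camp game mode that drives the in-game clock.
; Each tick it checks every BP_Person and advances time only while all of them have TaskWorking set.
; When time advances, it adds scaled delta seconds to TimeOfDay and broadcasts OnTimeUpdated with the new time and step.
; The current TimeOfDay prints on screen every frame as debug output.
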(event EventTick
  (params (DeltaSeconds :type Float%20%28single-precision%29))
  (bind _timespeed (Variables|Default|GetTimeSpeed))
  (bind _returnvalue (* _timespeed DeltaSeconds))
  (bind _outactors (Actor|GetAllActorsOfClass "/Game/Island/Blueprints/BP_Person.BP_Person_C"))
  (Variables|Default|SetTimeTicking true)
  (bind _array_element (Utilities|Array|ForEachLoopwithBreak _outactors :!label _label)
    (:LoopBody
      (Utilities|IsValid _array_element
        (:Is%20Valid
          (if (not (Variables|/Game/Island/Blueprints/BP_Person.BP_Person_C|GetTaskWorking _array_element))
            (Variables|Default|SetTimeTicking false)
            (goto _label Break)))))
    (:Completed
      (if (Variables|Default|GetTimeTicking)
        (bind _output_get (Variables|Default|SetTimeOfDay (+ (Variables|Default|GetTimeOfDay) _returnvalue)))
        (Default|CallOnTimeUpdated _output_get _returnvalue))
      (Development|PrintString (Utilities|String|ToString(Float) (Variables|Default|GetTimeOfDay)) true false "(R=1.000000,G=0.072449,B=0.959508,A=1.000000)" 0.0))))

(event EventBeginPlay)

(fn ConstructionScript)