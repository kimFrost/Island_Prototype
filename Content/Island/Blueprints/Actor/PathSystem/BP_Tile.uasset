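; Island path-system tile actor that clears foliage around itself when revealed and displays its distance from the selected person.
; On its reveal event, a sphere multi-trace with persistent debug drawing finds foliage instanced mesh components and removes the hit instances.
; The game instance's reveal event only prints a debug message.
; Construction creates a dynamic material with a black Color parameter, and Tick refreshes the distance text.
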(event Custom|CustomEvent_0
  (params (Tile :type Island%20Tile%20Object%20Reference))
  (bind _returnvalue (Transformation|GetActorLocation))
  (Development|PrintString "Hello" true true "(R=0.000000,G=0.660000,B=1.000000,A=1.000000)" 2e+01)
  (bind (_outhits _returnvalue_2) (Class|KismetSystemLibrary|SphereTraceMultiNEW (+ _returnvalue "0, 0,1.000000") (- _returnvalue "0, 0,1.000000") 4e+02 "TraceTypeQuery3" true 0 "Persistent" true))
  (if _returnvalue_2
    (for _array_element _outhits
      (bind _asfoliage_instanced_static_mesh_component (Utilities|Casting|CastToFoliageInstancedStaticMeshComponent (.HitComponent (Collision|BreakHitResult _array_element))))
      (Class|InstancedStaticMeshComponent|RemoveInstance _asfoliage_instanced_static_mesh_component (.HitItem (Collision|BreakHitResult _array_element))))))

(event Custom|CustomEvent_2
  (params (Tile :type Island%20Tile%20Object%20Reference))
  (Development|PrintString "reveal game isntance"))

(event EventBeginPlay
  (EventDispatchers|BindEventtoOnTileRevealed (delegate Custom|CustomEvent_0))
  (bind _asisland_game_instance (Utilities|Casting|CastToIslandGameInstance (Game|GetGameInstance)))
  (EventDispatchers|BindEventtoOnTileRevealed _asisland_game_instance (delegate Custom|CustomEvent_2)))

(event EventActorBeginOverlap
  (params (OtherActor :type Actor%20Object%20Reference)))

(event EventTick
  (params (DeltaSeconds :type Float%20%28single-precision%29))
  (Rendering|Components|TextRender|SetText (Variables|Default|GetTextRender) (Utilities|Text|ToText(Integer) (Variables|Default|GetDistanceFromSelectedPerson))))

(fn ConstructionScript
  (bind _basemesh (Variables|Default|GetBaseMesh))
  (|CallParentFunction)
  (Utilities|FlowControl|Sequence
    (:then_1
      (Rendering|Material|SetMaterial _basemesh 1 0)
      (bind _returnvalue (Rendering|Material|CreateDynamicMaterialInstance (Variables|Default|GetBaseMesh) 1 (Rendering|Material|GetMaterial _basemesh 1) :!class /Script/Engine.PrimitiveComponent))
      (bind _output_get (Variables|Default|SetDynamicMaterial _returnvalue))
      (Rendering|Material|SetVectorParameterValue _output_get "Color" "(R=0.000000,G=0.000000,B=0.000000,A=1.000000)" :!class /Script/Engine.MaterialInstanceDynamic))))