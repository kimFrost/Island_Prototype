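; BP_Station is a work station actor in the island camp game, where assigned people perform the task defined by its row data.
; Construction gathers child C_StationSlot components; functions find a free slot and start an arriving person working on the station's task.
; Widgets show title, task progress, a screen-bounds-sized space area, and possible outcomes when hovering with Select and a selected person.
; An older outcome-processing event remains, its binding disconnected.
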(event Custom|_OnProcessStations
  ;[1 0 0.01317] Old
  (for _array_element (Variables|Default|GetStationSlots)
    (Utilities|IsValid (Variables|/Game/Island/Blueprints/Actor/Components/C_StationSlot.C_StationSlot_C|GetAsignedPerson _array_element)
      (:Is%20Valid
        (bind _asgi_island (Utilities|Casting|CastToGI_Island (Game|GetGameInstance)))
        (bind _array_element_2 (Utilities|Array|ForEachLoopwithBreak 0 :!label _label)
          (:LoopBody
            (if (Math|Float|InRange(Float) 0.6 (.ChanceRangeFrom (Utilities|Struct|BreakST_Outcome _array_element_2)) (.ChanceRangeTo (Utilities|Struct|BreakST_Outcome _array_element_2)))
              (Class|IslandGameInstance|ParseOutcome _asgi_island _array_element_2 (Variables|/Game/Island/Blueprints/Actor/Components/C_StationSlot.C_StationSlot_C|GetAsignedPerson _array_element) "Work" true)
              (goto _label Break))))))))

(event EventBeginPlay
  (bind _aswidget_label (Utilities|Casting|CastToWidget_Label (UserInterface|GetUserWidgetObject (Variables|Default|GetLabelWidget))))
  (Variables|/Game/Island/Blueprints/Widgets/Widget_Label.Widget_Label_C|SetTitle _aswidget_label (.Title (Utilities|Struct|BreakST_Station (Variables|Default|GetStationRowData)))))

(event EventTick
  (params (DeltaSeconds :type Float%20%28single-precision%29))
  (Utilities|FlowControl|Sequence
    (:then_0
      ;[1 1 1] Set space widget size
      (bind _aspc_camp_controller (Utilities|Casting|CastToPC_CampController (Game|GetPlayerController 0)))
      (Class|WidgetComponent|SetDrawSize (Variables|Default|GetSpaceWidget) (/ (- (.Max (Utilities|Struct|BreakBox2D (Class|IslandPlayerControllerBase|GetObjectScreenBounds _aspc_camp_controller self))) (.Min (Utilities|Struct|BreakBox2D (Class|IslandPlayerControllerBase|GetObjectScreenBounds _aspc_camp_controller self)))) (Class|WidgetLayoutLibrary|GetViewportScale))))
    (:then_1
      (bind _aswidget_progress (Utilities|Casting|CastToWidget_Progress (UserInterface|GetUserWidgetObject (Variables|Default|GetProgressWidget))))
      (Variables|/Game/Island/Blueprints/Widgets/Widget_Progress.Widget_Progress_C|SetProgress _aswidget_progress (Utilities|Struct|BreakST_Task (Variables|Default|GetCurrentTask))))))

(event MouseInput|EventActorEndCursorOver
  (Development|SetHiddeninGame (Variables|Default|GetOutcomesWidget) true false))

(event MouseInput|EventActorBeginCursorOver
  (bind _outcomeswidget (Variables|Default|GetOutcomesWidget))
  (bind _aspc_camp_controller (Utilities|Casting|CastToPC_CampController (Game|GetPlayerController 0)))
  (switch Utilities|FlowControl|Switch|SwitchonEnum_PCToolType (Variables|/Game/Island/Blueprints/PC_CampController.PC_CampController_C|GetToolType _aspc_camp_controller)
    (:NewEnumerator0
      (Utilities|IsValid (Variables|/Game/Island/Blueprints/PC_CampController.PC_CampController_C|GetSelectedPerson _aspc_camp_controller)
        (:Is%20Valid
          (Development|SetHiddeninGame _outcomeswidget false false)
          (bind _aswidget_outcomes (Utilities|Casting|CastToWidget_Outcomes (UserInterface|GetUserWidgetObject _outcomeswidget)))
          (Variables|/Game/Island/Blueprints/Widgets/Widget_Outcomes.Widget_Outcomes_C|SetOutcomes _aswidget_outcomes (.Outcomes (Utilities|Struct|BreakST_Task (.Task (Utilities|Struct|BreakST_Station (Variables|Default|GetStationRowData))))))
          (Variables|/Game/Island/Blueprints/Widgets/Widget_Outcomes.Widget_Outcomes_C|SetPerson _aswidget_outcomes (Variables|/Game/Island/Blueprints/PC_CampController.PC_CampController_C|GetSelectedPerson _aspc_camp_controller))
          (Default|Update _aswidget_outcomes))))))

(event MouseInput|EventActorOnClicked
  (params (ButtonPressed :type Key%20Structure :default "AnyKey")))

(fn ConstructionScript
  ;[1 1 1] Get all station slots and store in array
  (Utilities|Array|Clear (Variables|Default|GetStationSlots))
  (for _array_element (Components|GetChildrenComponents (VehicleSound|GetRootComponent) true)
    (bind _asc_station_slot (Utilities|Casting|CastToC_StationSlot _array_element))
    (Utilities|Array|Add (Variables|Default|GetStationSlots) _asc_station_slot)))

(fn GetFreeSlot
  (for _array_element (Variables|Default|GetStationSlots)
    (Class|IslandBlueprintFunctionLibrary|NotNull (Variables|/Game/Island/Blueprints/Actor/Components/C_StationSlot.C_StationSlot_C|GetAsignedPerson _array_element)
      (:Null
        (return _array_element))))
  (return 0))

(fn PersonArivedatStation
  (params (Person :type BP%20Person%20Object%20Reference))
  (bind _returnvalue (Class|IslandStation|GetTask))
  (bind _output_get (Variables|/Game/Island/Blueprints/BP_Person.BP_Person_C|SetTask Person _returnvalue))
  (Variables|/Script/Island_Prototype.IslandPerson|SetbIsWorking Person (> (.WorkTime (Utilities|Struct|BreakST_Task _output_get)) 0.0))
  (Development|SetHiddeninGame (Variables|Default|GetProgressWidget) false false)
  (Variables|/Script/Island_Prototype.IslandPerson|SetCurrentState Person "Working"))