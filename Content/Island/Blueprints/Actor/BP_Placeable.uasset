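; BP_Placeable is an island actor that keeps a list of assigned people, apparently as a base for placeable objects.
; RemovePerson removes a person from that list, with nothing acting on the result.
; PlacePerson only checks whether the person is already listed and never adds them.
; The events and construction script are empty, and the InConstructMode variable is unused.
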(event EventBeginPlay)

(event EventActorBeginOverlap
  (params (OtherActor :type Actor%20Object%20Reference)))

(event EventTick
  (params (DeltaSeconds :type Float%20%28single-precision%29)))

(fn ConstructionScript)

(fn PlacePerson
  (params (Person :type BP%20Person%20Object%20Reference))
  (if (Utilities|Array|ContainsItem (Variables|Default|GetAsignedPeople) Person)
    _))

(fn RemovePerson
  (params (Person :type BP%20Person%20Object%20Reference))
  (bind _returnvalue (Utilities|Array|RemoveItem (Variables|Default|GetAsignedPeople) Person))
  (if _returnvalue
    _))