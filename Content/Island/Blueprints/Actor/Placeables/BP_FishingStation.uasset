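; BP_FishingStation is a placeable island station that loads its StationRowData from the FishingStation row of DATA_Stations in the construction script.
; BeginPlay only calls the parent, so any live behaviour comes from the parent class.
; Disconnected leftover graphs would set a "Fishing" label, bind to GI_Island's station processing, and have assigned workers store random gathered items and log completed tasks, but none of them run.
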(event EventBeginPlay
  (|CallParentFunction))

(event Collision|EventActorBeginOverlap
  (params (OtherActor :type Actor%20Object%20Reference)))

(event EventTick
  (params (DeltaSeconds :type Float%20%28single-precision%29))
  (|CallParentFunction 0.0))

(fn ConstructionScript
  (|CallParentFunction)
  (bind _returnvalue (Utilities|GetDataTableRow "/Game/Island/Util/Structs/DATA_Stations.DATA_Stations" "FishingStation")
    (:then
      (Variables|Default|SetStationRowData _returnvalue))))