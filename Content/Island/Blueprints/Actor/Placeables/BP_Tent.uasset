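; BP_Tent is a placeable island actor representing a tent, described as a place to rest that improves privacy and comfort and reduces fatigue.
; On BeginPlay it runs the parent logic, casts the LabelWidget's user widget to Widget_Label, then sets the label's title and the tent's description and effect texts.
; The effects are display text only here, with no gameplay logic in this Blueprint's own graphs.
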(event EventBeginPlay
  (|CallParentFunction)
  (bind _aswidget_label (Utilities|Casting|CastToWidget_Label (UserInterface|GetUserWidgetObject (Variables|Default|GetLabelWidget))))
  (Variables|/Game/Island/Blueprints/Widgets/Widget_Label.Widget_Label_C|SetTitle _aswidget_label "Tent")
  (Variables|Default|SetDescription "A place to rest and get some time for one self.")
  (Variables|Default|SetEffectDescription "+Privacy 
+Comfort 
--Fatigue"))

(event Collision|EventActorBeginOverlap
  (params (OtherActor :type Actor%20Object%20Reference)))

(event EventTick
  (params (DeltaSeconds :type Float%20%28single-precision%29))
  (|CallParentFunction 0.0))

(fn ConstructionScript
  (|CallParentFunction))