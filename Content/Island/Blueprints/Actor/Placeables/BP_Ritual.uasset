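; BP_Ritual is a placeable island station where people perform rituals, advertised as adding Social and reducing Fatigue.
; BeginPlay sets its label and descriptions, then binds to GI_Island's OnProcessStations event.
; The handler loops over assigned station slots but only casts the game instance: no effect is applied, and a "relaxed by the fire" task log is left disconnected.
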(event Custom|_OnProcessStations
  (for _array_element (Variables|Default|GetStationSlots)
    (Utilities|IsValid (Variables|/Game/Island/Blueprints/Actor/Components/C_StationSlot.C_StationSlot_C|GetAsignedPerson _array_element)
      (:Is%20Valid
        (bind _asgi_island (Utilities|Casting|CastToGI_Island (Game|GetGameInstance)))))))

(event EventBeginPlay
  (|CallParentFunction)
  (bind _aswidget_label (Utilities|Casting|CastToWidget_Label (UserInterface|GetUserWidgetObject (Variables|Default|GetLabelWidget))))
  (Variables|/Game/Island/Blueprints/Widgets/Widget_Label.Widget_Label_C|SetTitle _aswidget_label "Ritual")
  (Variables|Default|SetDescription "A place to perform rituals")
  (Variables|Default|SetEffectDescription "+Social (if not alone at ritual) 
-Fatigue")
  (bind _asgi_island (Utilities|Casting|CastToGI_Island (Game|GetGameInstance)))
  (EventDispatchers|BindEventtoOnProcessStations _asgi_island (delegate Custom|_OnProcessStations)))

(event Collision|EventActorBeginOverlap
  (params (OtherActor :type Actor%20Object%20Reference)))

(event EventTick
  (params (DeltaSeconds :type Float%20%28single-precision%29)))

(fn ConstructionScript
  (|CallParentFunction)
  (if (Variables|Default|GetbInConstructMode)
    _))