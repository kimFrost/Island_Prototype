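; BP_CampExit is a camp placeable station, labelled "Explore", that decides which person is the island's explorer.
; On BeginPlay it sets the label widget title and binds to the GI_Island game instance's OnProcessStations event.
; When stations process, it writes the first slot's assigned person to the game instance's Explorer, or clears it if none.
; An unconnected loop that would gather every slot's person into ExploreGroup never runs.
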(event Custom|_OnProcessStations
  (bind _stationslots (Variables|Default|GetStationSlots))
  (bind _item (Utilities|Array|Get(acopy) _stationslots))
  (bind _asignedperson (Variables|/Game/Island/Blueprints/Actor/Components/C_StationSlot.C_StationSlot_C|GetAsignedPerson _item))
  (Utilities|IsValid _item
    (:Is%20Valid
      (Utilities|IsValid _asignedperson
        (:Is%20Valid
          (bind _asgi_island (Utilities|Casting|CastToGI_Island (Game|GetGameInstance)))
          (Variables|/Game/Island/Blueprints/GI_Island.GI_Island_C|SetExplorer _asgi_island _asignedperson))
        (:Is%20Not%20Valid
          (bind _asgi_island_2 (Utilities|Casting|CastToGI_Island (Game|GetGameInstance) :!label _label))
          (Variables|/Game/Island/Blueprints/GI_Island.GI_Island_C|SetExplorer _asgi_island_2 0))))
    (:Is%20Not%20Valid
      (goto _label))))

(event EventBeginPlay
  (|CallParentFunction)
  (bind _aswidget_label (Utilities|Casting|CastToWidget_Label (UserInterface|GetUserWidgetObject (Variables|Default|GetLabelWidget))))
  (Variables|/Game/Island/Blueprints/Widgets/Widget_Label.Widget_Label_C|SetTitle _aswidget_label "Explore")
  (bind _asgi_island (Utilities|Casting|CastToGI_Island (Game|GetGameInstance)))
  (EventDispatchers|BindEventtoOnProcessStations _asgi_island (delegate Custom|_OnProcessStations)))

(event EventActorBeginOverlap
  (params (OtherActor :type Actor%20Object%20Reference)))

(event EventTick
  (params (DeltaSeconds :type Float%20%28single-precision%29))
  (|CallParentFunction 0.0))

(fn ConstructionScript
  (|CallParentFunction))